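; Customer group actor for a VR Dinner Dash game, representing one party from selection and seating to departure.
; Motion controller overlap shows the pointer and enables input, so releasing select toggles the group's highlight and CustomerSpawner selection.
; Lifecycle events update the Table and send heart-scaled scores to the Podium, compounding the stored multiplier on each award.
; Leaving happy or sad removes the group from the spawner and table, then destroys its figures and itself.
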(event `self.ReceiveBeginPlay`
  ;[1 1 1] Set initial values and handle start logic
  (`self.SetInitialValues`))

(event `self.customerCollider.OnComponentBeginOverlap`
  (params (OverlappedComponent :type "PrimitiveComponent Object Reference") (OtherActor :type "Actor Object Reference") (OtherComp :type "PrimitiveComponent Object Reference") (OtherBodyIndex :type Integer) (bFromSweep :type Boolean) (SweepResult :type "HitResult Structure (by ref)"))
  ;[1 1 1] Check if user is pointing at customer
  (bind _asbp_motion_controller (cast `/Game/VirtualRealityBP/Blueprints/BP_MotionController` OtherActor))
  (`/Engine/EditorBlueprintResources/StandardMacros.IsValid` _asbp_motion_controller
    (:`Is Valid`
      (`self.EnableInput` (`GameplayStatics.GetPlayerController` 0))
      (`SceneComponent.SetVisibility` (`/Game/VirtualRealityBP/Blueprints/BP_MotionController.pointer` _asbp_motion_controller) true false)
      (switch `EControllerHand` (`/Game/VirtualRealityBP/Blueprints/BP_MotionController.Hand` _asbp_motion_controller)
        (:`Left`
          (set `self.leftPointing` true))
        (:`Right`
          (set `self.rightPointing` true))))))

(event `self.customerCollider.OnComponentEndOverlap`
  (params (OverlappedComponent :type "PrimitiveComponent Object Reference") (OtherActor :type "Actor Object Reference") (OtherComp :type "PrimitiveComponent Object Reference") (OtherBodyIndex :type Integer))
  ;[1 1 1] Check if user is pointing at customer
  (bind _asbp_motion_controller (cast `/Game/VirtualRealityBP/Blueprints/BP_MotionController` OtherActor))
  (`/Engine/EditorBlueprintResources/StandardMacros.IsValid` _asbp_motion_controller
    (:`Is Valid`
      (`self.DisableInput` (`GameplayStatics.GetPlayerController` 0))
      (`SceneComponent.SetVisibility` (`/Game/VirtualRealityBP/Blueprints/BP_MotionController.pointer` _asbp_motion_controller) false false)
      (switch `EControllerHand` (`/Game/VirtualRealityBP/Blueprints/BP_MotionController.Hand` _asbp_motion_controller)
        (:`Left`
          (set `self.leftPointing` false))
        (:`Right`
          (set `self.rightPointing` false))))))

(event `InputAction|SelectLeft`
  (params (Key :type "Key Structure"))
  (bind _customerspawner (`self.customerSpawner`))
  ;[1 1 1] Handle Highlight for customer if user selected customer or not
  (:`Released`
    (if (`self.leftPointing`)
      (bind _output_get (set `self.groupHighlighted` (not (`self.groupHighlighted`)) :!label _label))
      (`self.HighlightGroup` _output_get)
      (if _output_get
        (`/Game/VR_DinnerDash_Assets/BP/BP_CustomerSpawner.SetSelectedCustomer` _customerspawner self)
        (else
          (`/Game/VR_DinnerDash_Assets/BP/BP_CustomerSpawner.SetSelectedCustomer` _customerspawner null))))))

(event `InputAction|SelectRight`
  (params (Key :type "Key Structure"))
  ;[1 1 1] Handle Highlight for customer if user selected customer or not
  (:`Released`
    (if (`self.rightPointing`)
      (goto _label))))

(event `self.OnCustomerSeated`
  ;[1 1 1] Handle Customer Events
  (`self.CalculateSeatingScore`))

(event `self.OnCustomerReadyToOrder`
  ;[1 1 1] Handle Customer Events
  (`/Game/VR_DinnerDash_Assets/BP/BP_Table.SpawnFoodOrder` (`self.table`)))

(event `self.OnCustomerOrderReceived`
  ;[1 1 1] Handle Customer Events
  (`/Game/VR_DinnerDash_Assets/BP/BP_Table.ShowTableNumber` (`self.table`) true)
  (`self.Apply FInal Score` (`self.foodItemScore`)))

(event `self.OnCustomerFoodReceived`
  ;[1 1 1] Handle Customer Events
  (`/Game/VR_DinnerDash_Assets/BP/BP_Table.ShowTableNumber` (`self.table`) false)
  (`self.Apply FInal Score` (`self.foodOrderScore`)))

(event `self.OnCustomerReadyToLeave`
  ;[1 1 1] Handle Customer Events
  (`/Game/VR_DinnerDash_Assets/BP/BP_Table.SpawnDirtyDishes` (`self.table`))
  (`self.Apply FInal Score` (`self.customerLeaveScore`)))

(event `self.OnCustomerLeaveHappy`
  ;[1 1 1] Handle Customer Events
  (`self.Apply FInal Score` (`self.customerLeaveScore`))
  (`self.DestroyCustomers` :!label _label_2))

(event `self.OnCustomerLeaveSad`
  ;[1 1 1] Handle Customer Events
  (goto _label_2))

(event `self.OnHeartRemoved`
  ;[1 1 1] Handle Customer Events
  (`self.ProcessRemovedHeart`))

(fn `Apply FInal Score`
  (params (`raw Score` :type Integer))
  (locals (scoreMultiplier :type "Float (double-precision)" :default 2.0) (scoreModifier :type "Float (double-precision)"))
  (bind _output_get (set `local.scoreModifier` (/ (`KismetMathLibrary.Conv_IntToDouble` (`self.customerHearts`)) (`KismetMathLibrary.Conv_IntToDouble` (`self.maxHearths`)))))
  (bind _output_get_2 (set `local.scoreMultiplier` (* _output_get (`local.scoreMultiplier`))))
  (`/Game/VR_DinnerDash_Assets/BP/BP_Podium.AddScore` (`self.podium`) (`KismetMathLibrary.FTrunc` (* `raw Score` _output_get_2))))

(fn `CalculateSeatingScore`
  (locals (scoreToAdd :type Integer))
  (bind _output_get (set `local.scoreToAdd` (* (`self.seatingScore`) (`BlueprintSetLibrary.Set_Length` (`self.listOfCustomers`)))))
  (`self.Apply FInal Score` _output_get))

(fn `DestroyCustomers`
  (bind _table (`self.table`))
  ;[1 1 1] Go through each customer figure and destroy it, afterwars destroy the customer actor
  (`/Game/VR_DinnerDash_Assets/BP/BP_CustomerSpawner.RemoveCustomerInLine` (`self.customerSpawner`) self)
  (`|ExecutionSequence`
    (:`then_0`
      (if (`KismetSystemLibrary.IsValid` _table)
        (set `/Game/VR_DinnerDash_Assets/BP/BP_Table.customerInTable` null _table)))
    (:`then_1`
      (bind _result (`BlueprintSetLibrary.Set_ToArray` (`self.listOfCustomers`)))
      (for _array_element _result
        (`self.K2_DestroyActor` _array_element))
      (`self.K2_DestroyActor`))))

(fn `HighlightGroup`
  (params (highlightState :type Boolean))
  (bind _listofcustomers (`self.listOfCustomers`))
  ;[1 1 1] Go through each customer figure and highligh them
  (for _index (range (+ (`BlueprintSetLibrary.Set_Length` _listofcustomers) 1))
    (bind _result (`BlueprintSetLibrary.Set_ToArray` _listofcustomers))
    (bind _asbp_customer_figure (cast `/Game/VR_DinnerDash_Assets/BP/BP_Customer_Figure` (`|GetArrayItem` _result _index)))
    (`/Game/VR_DinnerDash_Assets/BP/BP_Customer_Figure.HighlightCustomer` _asbp_customer_figure highlightState)))

(fn `ProcessRemovedHeart`
  ;[1 1 1] Update heart meter
  (`TextRenderComponent.K2_SetText` (`self.customerHeartCounter`) (`KismetTextLibrary.Conv_IntToText` (`self.customerHearts`))))

(fn `SetInitialValues`
  ;[1 1 1] Set initial values for customer
  (`|ExecutionSequence`
    (:`then_0`
      (set `self.customerFigureReference` "/Game/VR_DinnerDash_Assets/BP/BP_Customer_Figure.BP_Customer_Figure_C"))
    (:`then_1`
      (bind _output_get (set `self.customerHearts` 10))
      (set `self.maxHearths` _output_get))
    (:`then_2`
      (set `self.customerPatience` 10.0))
    (:`then_3`
      (set `self.lookAtMenuTime` 10.0))
    (:`then_4`
      (set `self.eatingTime` 10.0))
    (:`then_5`
      (bind _returnvalue (`GameplayStatics.GetActorOfClass` "/Game/VR_DinnerDash_Assets/BP/BP_CustomerSpawner.BP_CustomerSpawner_C"))
      (set `self.customerSpawner` _returnvalue))
    (:`then_6`
      (bind _returnvalue_2 (`GameplayStatics.GetActorOfClass` "/Game/VR_DinnerDash_Assets/BP/BP_Podium.BP_Podium_C"))
      (set `self.podium` _returnvalue_2))))

(fn `UserConstructionScript`)