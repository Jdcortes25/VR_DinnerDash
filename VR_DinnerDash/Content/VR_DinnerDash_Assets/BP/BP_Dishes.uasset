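; BP_Dishes is a dish actor for a VR dinner game that motion controllers can pick up and drop.
; Pickup turns off physics and collision, attaches the dish to the hand component and, if a Customer reference is valid, calls CustomerLeave on it.
; Drop detaches the dish and restores physics and collision.
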(event `/Game/VirtualRealityBP/Blueprints/PickupActorInterface.Pickup`
  (params (AttachTo :type "SceneComponent Object Reference"))
  (bind _customer (`self.customer`))
  (`PrimitiveComponent.SetSimulatePhysics` (`self.Dish_Mesh`) false)
  (`SceneComponent.K2_AttachToComponent` (`self.K2_GetRootComponent`) AttachTo "None" "KeepWorld" "KeepWorld" "KeepWorld" false)
  (`PrimitiveComponent.SetCollisionEnabled` (`self.Dish_Mesh`) "NoCollision")
  (if (`KismetSystemLibrary.IsValid` _customer)
    (`CustomerActor.CustomerLeave` _customer true)))

(event `/Game/VirtualRealityBP/Blueprints/PickupActorInterface.Drop`
  (`PrimitiveComponent.SetSimulatePhysics` (`self.Dish_Mesh`) true)
  (`self.K2_DetachFromActor` "KeepWorld" "KeepWorld" "KeepWorld")
  (`PrimitiveComponent.SetCollisionEnabled` (`self.Dish_Mesh`) "QueryAndPhysics"))

(fn `UserConstructionScript`)