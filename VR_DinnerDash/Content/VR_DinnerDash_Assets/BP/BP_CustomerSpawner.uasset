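; BP_CustomerSpawner spawns customers into a spaced waiting line in VR Dinner Dash and tracks which customer is selected.
; It spawns one on BeginPlay, then Tick sets a timer with a randomly picked cooldown whenever the line has room and no spawn is pending.
; Customers attach to the spawner and are respaced along local Y when one is removed.
; Selecting a new customer clears the previous customer's group highlight.
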(event `self.ReceiveBeginPlay`
  ;[1 1 1] Spawn a Customer on start of the game
  (`self.SpawnCustomer`))

(event `self.ReceiveTick`
  (params (DeltaSeconds :type "Float (single-precision)"))
  ;[1 1 1] Update
  (`self.PrepareToSpawnCustomer`))

(fn `PrepareToSpawnCustomer`
  (bind _spawncooldowns (`self.spawnCooldowns`))
  ;[1 1 1] Set timed event for when to spawn new customer
  (if (and (not (`self.waitingToSpawn`)) (< (`BlueprintSetLibrary.Set_Length` (`self.customerLine`)) (`self.maxAmountOfCustomers`)))
    (set `self.cooldownTime` (`|GetArrayItem` _spawncooldowns (`KismetMathLibrary.RandomIntegerInRange` 0 (- (`KismetArrayLibrary.Array_Length` _spawncooldowns) 1))))
    (set `self.waitingToSpawn` true)
    (`KismetSystemLibrary.K2_SetTimer` null "SpawnCustomer" (`KismetMathLibrary.Conv_IntToDouble` (`self.cooldownTime`)))))

(fn `RemoveCustomerInLine`
  (params (customer :type "/Game/VR_DinnerDash_Assets/BP/BP_Customer Object Reference"))
  ;[1 1 1] Remove the customer from the line and update the line so that customers are spaces correctly
  (`BlueprintSetLibrary.Set_Remove` (`self.customerLine`) customer)
  (`self.UpdatePositionsInLine`))

(fn `SetSelectedCustomer`
  (params (newSelectedCustomer :type "/Game/VR_DinnerDash_Assets/BP/BP_Customer Object Reference"))
  (bind _selectedcustomer (`self.selectedCustomer`))
  ;[1 1 1] Set selected customer, unhighlight previous selected customer and unhighlight new selected customer
  (if (`KismetSystemLibrary.IsValid` _selectedcustomer)
    (bind _output_get (set `/Game/VR_DinnerDash_Assets/BP/BP_Customer.groupHighlighted` false _selectedcustomer))
    (`/Game/VR_DinnerDash_Assets/BP/BP_Customer.HighlightGroup` _selectedcustomer _output_get))
  (set `self.selectedCustomer` newSelectedCustomer))

(fn `SpawnCustomer`
  (bind _customerline (`self.customerLine`))
  ;[1 1 1] Spawn a customer and place them accordingly in the waiting line
  (set `self.locationToSpawn` (`KismetMathLibrary.MakeVector` 0.0 (* (`BlueprintSetLibrary.Set_Length` _customerline) (`self.customerSpacing`))))
  (bind _returnvalue (`|SpawnActorFromClass` "/Game/VR_DinnerDash_Assets/BP/BP_Customer.BP_Customer_C" (`KismetMathLibrary.MakeTransform` (`self.locationToSpawn`)) "Undefined" "OverrideRootScale" null null))
  (`BlueprintSetLibrary.Set_Add` _customerline _returnvalue)
  (`self.K2_AttachToActor` _returnvalue self "None" "KeepRelative" "KeepRelative" "KeepRelative" true)
  (set `self.waitingToSpawn` false))

(fn `UpdatePositionsInLine`
  ;[1 1 1] Update the waiting line so that all customers are spaced correctly
  (bind _result (`BlueprintSetLibrary.Set_ToArray` (`self.customerLine`)))
  (for (_array_element _array_index) _result
    (`self.K2_SetActorRelativeLocation` _array_element (`KismetMathLibrary.MakeVector` 0.0 (* _array_index (`self.customerSpacing`))) false false)))

(fn `UserConstructionScript`)