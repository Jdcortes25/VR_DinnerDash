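; BP_FoodItem is a VR food plate that a motion controller can pick up and drop.
; Pickup disables physics and collision on the plate mesh and attaches the actor to the given component, keeping world transform.
; The first pickup also removes the item from its FoodStation's list, guarded by a HasBeenPickedUp flag.
; Drop restores simulation and collision and detaches the actor.
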(event `/Game/VirtualRealityBP/Blueprints/PickupActorInterface.Pickup`
  (params (AttachTo :type "SceneComponent Object Reference"))
  (`PrimitiveComponent.SetSimulatePhysics` (`self.Plate_MESH`) false)
  (`SceneComponent.K2_AttachToComponent` (`self.K2_GetRootComponent`) AttachTo "None" "KeepWorld" "KeepWorld" "KeepWorld" false)
  (`PrimitiveComponent.SetCollisionEnabled` (`self.Plate_MESH`) "NoCollision")
  (if (not (`self.hasBeenPickedUp`))
    (`/Game/VR_DinnerDash_Assets/BP/BP_FoodStation.Remove Food from List` (`self.foodStation`) self)
    (set `self.hasBeenPickedUp` true)))

(event `/Game/VirtualRealityBP/Blueprints/PickupActorInterface.Drop`
  (`PrimitiveComponent.SetSimulatePhysics` (`self.Plate_MESH`) true)
  (`self.K2_DetachFromActor` "KeepWorld" "KeepWorld" "KeepWorld")
  (`PrimitiveComponent.SetCollisionEnabled` (`self.Plate_MESH`) "QueryAndPhysics"))

(fn `UserConstructionScript`)