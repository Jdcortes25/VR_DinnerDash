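; BP_Podium is the game manager for a VR dinner-service game, tracking score, stars and whether play is in progress.
; On BeginPlay it caches all tables, the customer spawner and the PodiumMenu widget, which it updates directly.
; StartGame restores stars, zeroes score after writing its text, and spawns a customer; StopGame resets tables and clears the spawner.
; RemoveStar hides star icons, but its zero-star StopGame check is unconnected.
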(event `self.ReceiveBeginPlay`
  (`self.SetInitialValues`))

(fn `AddScore`
  (params (points :type Integer))
  (bind _output_get (set `self.score` (+ points (`self.score`))))
  (`TextBlock.SetText` (`/Game/VR_DinnerDash_Assets/BP/PodiumMenu.scoreValue` (`self.podiumMenu`)) (`KismetTextLibrary.Conv_IntToText` _output_get)))

(fn `RemoveStar`
  (bind _podiummenu (`self.podiumMenu`))
  (bind _output_get (set `self.stars` (- (`self.stars`) 1)))
  (switch `int` _output_get
    (:`0`
      (`Widget.SetVisibility` (`/Game/VR_DinnerDash_Assets/BP/PodiumMenu.star_0` _podiummenu) "Hidden"))
    (:`1`
      (`Widget.SetVisibility` (`/Game/VR_DinnerDash_Assets/BP/PodiumMenu.star_1` _podiummenu) "Hidden"))
    (:`2`
      (`Widget.SetVisibility` (`/Game/VR_DinnerDash_Assets/BP/PodiumMenu.star_2` _podiummenu) "Hidden"))
    (:`3`
      (`Widget.SetVisibility` (`/Game/VR_DinnerDash_Assets/BP/PodiumMenu.star_3` _podiummenu) "Hidden"))
    (:`4`
      (`Widget.SetVisibility` (`/Game/VR_DinnerDash_Assets/BP/PodiumMenu.star_4` _podiummenu) "Hidden"))))

(fn `SetInitialValues`
  (`|ExecutionSequence`
    (:`then_0`
      (bind _outactors (`GameplayStatics.GetAllActorsOfClass` "/Game/VR_DinnerDash_Assets/BP/BP_Table.BP_Table_C"))
      (set `self.listOfTables` _outactors))
    (:`then_1`
      (set `self.initialStars` (`self.stars`)))
    (:`then_2`
      (bind _returnvalue (`GameplayStatics.GetActorOfClass` "/Game/VR_DinnerDash_Assets/BP/BP_CustomerSpawner.BP_CustomerSpawner_C"))
      (set `self.customerSpawner` _returnvalue))
    (:`then_3`
      (bind _foundwidgets (`WidgetBlueprintLibrary.GetAllWidgetsOfClass` "/Game/VR_DinnerDash_Assets/BP/PodiumMenu.PodiumMenu_C" false))
      (set `self.podiumMenu` (`|GetArrayItem` _foundwidgets)))))

(fn `StartGame`
  (bind _podiummenu (`self.podiumMenu`))
  (`|ExecutionSequence`
    (:`then_0`
      (set `self.gameInProgress` true)
      (`TextBlock.SetText` (`/Game/VR_DinnerDash_Assets/BP/PodiumMenu.scoreValue` (`self.podiumMenu`)) (`KismetTextLibrary.Conv_IntToText` (stale _output_get))))
    (:`then_1`
      (bind _output_get (set `self.score` 0)))
    (:`then_2`
      (set `self.stars` (`self.initialStars`))
      (`Widget.SetVisibility` (`/Game/VR_DinnerDash_Assets/BP/PodiumMenu.star_0` _podiummenu) "Visible")
      (`Widget.SetVisibility` (`/Game/VR_DinnerDash_Assets/BP/PodiumMenu.star_1` _podiummenu) "Visible")
      (`Widget.SetVisibility` (`/Game/VR_DinnerDash_Assets/BP/PodiumMenu.star_2` _podiummenu) "Visible")
      (`Widget.SetVisibility` (`/Game/VR_DinnerDash_Assets/BP/PodiumMenu.star_3` _podiummenu) "Visible")
      (`Widget.SetVisibility` (`/Game/VR_DinnerDash_Assets/BP/PodiumMenu.star_4` _podiummenu) "Visible"))
    (:`then_3`
      (`/Game/VR_DinnerDash_Assets/BP/BP_CustomerSpawner.SpawnCustomer` (`self.customerSpawner`)))))

(fn `StopGame`
  (bind _customerspawner (`self.customerSpawner`))
  (`|ExecutionSequence`
    (:`then_0`
      (set `self.gameInProgress` false))
    (:`then_1`
      (for _array_element (`self.listOfTables`)
        (`/Game/VR_DinnerDash_Assets/BP/BP_Table.ResetTable` _array_element)))
    (:`then_2`
      (`/Game/VR_DinnerDash_Assets/BP/BP_CustomerSpawner.StopSpawner` _customerspawner)
      (`/Game/VR_DinnerDash_Assets/BP/BP_CustomerSpawner.ClearCustomerLine` _customerspawner))))

(fn `UserConstructionScript`)