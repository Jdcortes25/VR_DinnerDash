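; BP_Table is a VR restaurant table that seats customer parties, takes their food and holds their dirty dishes.
; Motion controller overlap previews the spawner's selected party over free chairs by re-parenting figures; releasing Select seats them, leaving returns them to the line.
; Overlapping food items with a matching table number are destroyed and reported to the customer.
; It also spawns orders and dishes, toggles its number indicator, and clears everything on reset.
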(event `self.ReceiveBeginPlay`
  (`self.SetInitialValues`))

(event `self.Table Collider.OnComponentBeginOverlap`
  (params (OverlappedComponent :type "PrimitiveComponent Object Reference") (OtherActor :type "Actor Object Reference") (OtherComp :type "PrimitiveComponent Object Reference") (OtherBodyIndex :type Integer) (bFromSweep :type Boolean) (SweepResult :type "HitResult Structure (by ref)"))
  (bind _asbp_motion_controller (cast `/Game/VirtualRealityBP/Blueprints/BP_MotionController` OtherActor)
    (:`then`
      (`/Engine/EditorBlueprintResources/StandardMacros.IsValid` _asbp_motion_controller
        (:`Is Valid`
          (`self.SelectTable` _asbp_motion_controller true))))
    (:`CastFailed`
      (bind _asbp_food_item (cast `/Game/VR_DinnerDash_Assets/BP/BP_FoodItem` OtherActor))
      (`/Engine/EditorBlueprintResources/StandardMacros.IsValid` _asbp_food_item
        (:`Is Valid`
          (`self.ReceiveFood` _asbp_food_item))))))

(event `self.Table Collider.OnComponentEndOverlap`
  (params (OverlappedComponent :type "PrimitiveComponent Object Reference") (OtherActor :type "Actor Object Reference") (OtherComp :type "PrimitiveComponent Object Reference") (OtherBodyIndex :type Integer))
  (bind _asbp_motion_controller (cast `/Game/VirtualRealityBP/Blueprints/BP_MotionController` OtherActor))
  (`/Engine/EditorBlueprintResources/StandardMacros.IsValid` _asbp_motion_controller
    (:`Is Valid`
      (`self.SelectTable` _asbp_motion_controller))))

(event `InputAction|SelectLeft`
  (params (Key :type "Key Structure"))
  (:`Released`
    (if (`self.tableSelected`) :!label _label
      (`self.SeatCustomers`))))

(event `InputAction|SelectRight`
  (params (Key :type "Key Structure"))
  (:`Released`
    (goto _label)))

(fn `BringCustomersBackToLine`
  (bind _customerspawner (`self.customerSpawner`))
  (bind _customerspawner_2 (`self.customerSpawner`))
  (bind _selectedcustomer (`/Game/VR_DinnerDash_Assets/BP/BP_CustomerSpawner.selectedCustomer` _customerspawner))
  (bind _selectedcustomer_2 (`/Game/VR_DinnerDash_Assets/BP/BP_CustomerSpawner.selectedCustomer` _customerspawner_2))
  ;[1 1 1] Set the customer back to their initial position and put them back in the waiting line
  (bind _result (`BlueprintSetLibrary.Set_ToArray` (`CustomerActor.listOfCustomers` _selectedcustomer_2)))
  (for _array_element _result
    (bind _asbp_customer_figure (cast `/Game/VR_DinnerDash_Assets/BP/BP_Customer_Figure` _array_element))
    (`self.K2_SetActorRelativeTransform` _asbp_customer_figure (`/Game/VR_DinnerDash_Assets/BP/BP_Customer_Figure.initialTransform` _asbp_customer_figure) false false)
    (`self.K2_AttachToActor` _asbp_customer_figure _selectedcustomer_2 "None" "KeepRelative" "KeepRelative" "KeepRelative" true))
  (`self.K2_AttachToActor` _selectedcustomer_2 _customerspawner_2 "None" "KeepRelative" "KeepRelative" "KeepRelative" true)
  (bind _result_2 (`BlueprintSetLibrary.Set_ToArray` (`/Game/VR_DinnerDash_Assets/BP/BP_CustomerSpawner.customerLine` _customerspawner)))
  (`self.K2_SetActorRelativeTransform` _selectedcustomer (`KismetMathLibrary.MakeTransform` (`KismetMathLibrary.MakeVector` 0.0 (* (`KismetArrayLibrary.Array_Find` _result_2 _selectedcustomer) (`/Game/VR_DinnerDash_Assets/BP/BP_CustomerSpawner.customerSpacing` _customerspawner)))) false false))

(fn `HoverCustomersOverChairs`
  (bind _selectedcustomer (`/Game/VR_DinnerDash_Assets/BP/BP_CustomerSpawner.selectedCustomer` (`self.customerSpawner`)))
  ;[1 1 1] Attach Customer Object to the table, move them above the table, attach individual customer figures to table and align them with a seat
  (`self.K2_AttachToActor` _selectedcustomer self "None" "KeepRelative" "KeepRelative" "KeepRelative" false)
  (`self.K2_SetActorRelativeLocation` _selectedcustomer (0.0 0.0 0.0) false false)
  (bind _result (`BlueprintSetLibrary.Set_ToArray` (`CustomerActor.listOfCustomers` _selectedcustomer)))
  (for _index (range (+ (`KismetArrayLibrary.Array_Length` _result) 1))
    (bind _output (`|GetArrayItem` _result _index))
    (if (`KismetSystemLibrary.IsValid` _output)
      (`self.K2_AttachToActor` _output self "None" "KeepRelative" "KeepRelative" "KeepRelative" false)
      (bind _returnvalue (`SceneComponent.GetRelativeTransform` (`/Game/VR_DinnerDash_Assets/BP/BP_Chair.DefaultSceneRoot` (`|GetArrayItem` (`self.chairs`) _index))))
      (`self.K2_SetActorRelativeTransform` _output (`KismetMathLibrary.MakeTransform` (`KismetMathLibrary.MakeVector` (.x (.location _returnvalue)) (.y (.location _returnvalue)) 100.0) (`KismetMathLibrary.MakeRotator` 0.0 0.0 (+ (.yaw (.rotation _returnvalue)) 90.0))) false false)
      (`self.K2_AttachToActor` _output _selectedcustomer "None" "KeepRelative" "KeepRelative" "KeepRelative" false))))

(fn `ReceiveFood`
  (params (foodItem :type "/Game/VR_DinnerDash_Assets/BP/BP_FoodItem Object Reference"))
  (if (`KismetStringLibrary.EqualEqual_StrStr` (`KismetTextLibrary.Conv_TextToString` (`TextRenderComponent.Text` (`/Game/VR_DinnerDash_Assets/BP/BP_FoodItem.Table Number` foodItem))) (`KismetStringLibrary.Conv_IntToString` (`self.tableNumber`)))
    (`self.K2_DestroyActor` foodItem)
    (`CustomerActor.FoodReceived` (`self.customerInTable`))))

(fn `ResetTable`
  (bind _foodorder (`self.foodOrder`))
  (bind _foodstation (`self.foodStation`))
  (bind _dirtydishes (`self.dirtyDishes`))
  (bind _customerintable (`self.customerInTable`))
  (`|ExecutionSequence`
    (:`then_0`
      ;[1 1 1] Destroy seating customer
      (`/Engine/EditorBlueprintResources/StandardMacros.IsValid` _customerintable
        (:`Is Valid`
          (`/Game/VR_DinnerDash_Assets/BP/BP_Customer.DestroyCustomers` _customerintable)
          (set `self.customerInTable` null))))
    (:`then_1`
      ;[1 1 1] Destroy food order
      (`/Engine/EditorBlueprintResources/StandardMacros.IsValid` _foodorder
        (:`Is Valid`
          (`self.K2_DestroyActor` _foodorder))))
    (:`then_2`
      ;[1 1 1] Hide table number indcator
      (`self.ShowTableNumber` false))
    (:`then_3`
      ;[1 1 1] Destroy Food Item
      (bind _fooditem (`/Game/VR_DinnerDash_Assets/BP/BP_FoodStation.GetFoodOrderByTableNumber` _foodstation (`self.tableNumber`)))
      (`/Engine/EditorBlueprintResources/StandardMacros.IsValid` _fooditem
        (:`Is Valid`
          (`|ExecutionSequence`
            (:`then_0`
              (`/Game/VR_DinnerDash_Assets/BP/BP_FoodStation.Remove Food from List` _foodstation _fooditem))
            (:`then_1`
              (`self.K2_DestroyActor` _fooditem))))))
    (:`then_4`
      ;[1 1 1] Destroy Dirty Dishes
      (`/Engine/EditorBlueprintResources/StandardMacros.IsValid` _dirtydishes
        (:`Is Valid`
          (`self.K2_DestroyActor` _dirtydishes))))))

(fn `SeatCustomers`
  (bind _customerspawner (`self.customerSpawner`))
  (bind _selectedcustomer (`/Game/VR_DinnerDash_Assets/BP/BP_CustomerSpawner.selectedCustomer` _customerspawner))
  (bind _selectedcustomer_2 (`/Game/VR_DinnerDash_Assets/BP/BP_CustomerSpawner.selectedCustomer` (`self.customerSpawner`)))
  ;[1 1 1] Handle Customer Seating Functionality
  (if (`KismetSystemLibrary.IsValid` _selectedcustomer_2)
    (if (and (not (`KismetSystemLibrary.IsValid` (`self.customerInTable`))) (<= (`BlueprintSetLibrary.Set_Length` (`CustomerActor.listOfCustomers` _selectedcustomer_2)) (`KismetArrayLibrary.Array_Length` (`self.chairs`))))
      (`|ExecutionSequence`
        (:`then_0`
          ;;[1 1 1] Table will be assigned to this customer, customer will be assigned to this customer, customer will be removed from the waiting line, and customer will no longer be selected
          (`|ExecutionSequence`
            (:`then_0`
              (set `self.customerInTable` _selectedcustomer))
            (:`then_1`
              (set `/Game/VR_DinnerDash_Assets/BP/BP_Customer.table` self _selectedcustomer))
            (:`then_2`
              (`/Game/VR_DinnerDash_Assets/BP/BP_CustomerSpawner.RemoveCustomerInLine` _customerspawner _selectedcustomer)
              (`/Game/VR_DinnerDash_Assets/BP/BP_CustomerSpawner.SetSelectedCustomer` _customerspawner null))
            (:`then_3`
              (`self.DisableInput` (`GameplayStatics.GetPlayerController` 0)))))
        (:`then_1`
          (bind _result (`BlueprintSetLibrary.Set_ToArray` (`CustomerActor.listOfCustomers` (`self.customerInTable`))))
          ;;[1 1 1] Loop through each customer figure and move them so they look as if they are sitting
          (for _array_element _result
            (bind _asbp_customer_figure (cast `/Game/VR_DinnerDash_Assets/BP/BP_Customer_Figure` _array_element))
            (bind _returnvalue (`SceneComponent.GetRelativeTransform` (`/Game/VR_DinnerDash_Assets/BP/BP_Customer_Figure.DefaultSceneRoot` _asbp_customer_figure)))
            (`self.K2_SetActorRelativeLocation` _asbp_customer_figure (`KismetMathLibrary.MakeVector` (.x (.location _returnvalue)) (.y (.location _returnvalue))) false false))
          ;;[1 1 1] Let customer know they have been seated
          (`CustomerActor.SeatCustomer` (`self.customerInTable`)))))))

(fn `SelectTable`
  (params (MotionController :type "/Game/VirtualRealityBP/Blueprints/BP_MotionController Object Reference") (selecting :type Boolean))
  (bind _returnvalue (`GameplayStatics.GetPlayerController` 0))
  (bind _selectedcustomer (`/Game/VR_DinnerDash_Assets/BP/BP_CustomerSpawner.selectedCustomer` (`self.customerSpawner`)))
  (bind _customercollider (`/Game/VR_DinnerDash_Assets/BP/BP_Customer.customerCollider` (`/Game/VR_DinnerDash_Assets/BP/BP_CustomerSpawner.selectedCustomer` (`self.customerSpawner`))))
  ;[1 1 1] Handle Selecting a table for customers
  (set `WidgetInteractionComponent.bShowDebug` selecting (`/Game/VirtualRealityBP/Blueprints/BP_MotionController.WidgetInteraction` MotionController))
  (if (`KismetSystemLibrary.IsValid` _selectedcustomer)
    (if (and (not (`KismetSystemLibrary.IsValid` (`self.customerInTable`))) (<= (`BlueprintSetLibrary.Set_Length` (`CustomerActor.listOfCustomers` _selectedcustomer)) (`KismetArrayLibrary.Array_Length` (`self.chairs`))))
      (set `self.tableSelected` selecting)
      (if selecting
        (`self.EnableInput` _returnvalue)
        (`PrimitiveComponent.SetCollisionEnabled` _customercollider "NoCollision")
        (`self.HoverCustomersOverChairs`)
        (else
          (`self.DisableInput` _returnvalue)
          (`PrimitiveComponent.SetCollisionEnabled` _customercollider "QueryOnly")
          (`self.BringCustomersBackToLine`))))))

(fn `SetInitialValues`
  ;[1 1 1] Set initial values
  (`|ExecutionSequence`
    (:`then_0`
      (bind _returnvalue (`GameplayStatics.GetActorOfClass` "/Game/VR_DinnerDash_Assets/BP/BP_CustomerSpawner.BP_CustomerSpawner_C"))
      (set `self.customerSpawner` _returnvalue)
      (bind _returnvalue_2 (`GameplayStatics.GetActorOfClass` "/Game/VR_DinnerDash_Assets/BP/BP_FoodStation.BP_FoodStation_C"))
      (set `self.foodStation` _returnvalue_2))
    (:`then_1`
      (for _array_element (`SceneComponent.GetChildrenComponents` (`self.Table Number Indicator`) false)
        (bind _astext_render_component (cast `TextRenderComponent` _array_element))
        (`TextRenderComponent.K2_SetText` _astext_render_component (`KismetTextLibrary.Conv_IntToText` (`self.tableNumber`)))
        (`SceneComponent.SetVisibility` (`self.Table Number Indicator`) false true)))))

(fn `ShowTableNumber`
  (params (visible :type Boolean))
  (`SceneComponent.SetVisibility` (`self.Table Number Indicator`) visible true))

(fn `SpawnDirtyDishes`
  (bind _returnvalue_location (`KismetMathLibrary.BreakTransform` (`SceneComponent.K2_GetComponentToWorld` (`self.ItemSpawnPoint`))))
  (bind _returnvalue (`|SpawnActorFromClass` "/Game/VR_DinnerDash_Assets/BP/BP_Dishes.BP_Dishes_C" (`KismetMathLibrary.MakeTransform` _returnvalue_location (struct) (0.6 0.6 0.01)) "Undefined" "OverrideRootScale" null null))
  (set `/Game/VR_DinnerDash_Assets/BP/BP_Dishes.customer` (`self.customerInTable`) _returnvalue)
  (set `self.dirtyDishes` _returnvalue))

(fn `SpawnFoodOrder`
  (bind _returnvalue_location (`KismetMathLibrary.BreakTransform` (`SceneComponent.K2_GetComponentToWorld` (`self.ItemSpawnPoint`))))
  ;[1 1 1] Spawn Food Order on the table
  (bind _returnvalue (`|SpawnActorFromClass` "/Game/VR_DinnerDash_Assets/BP/BP_FoodOrder.BP_FoodOrder_C" (`KismetMathLibrary.MakeTransform` _returnvalue_location (struct) (0.25 0.4 0.01)) "Undefined" "OverrideRootScale" null null))
  (set `/Game/VR_DinnerDash_Assets/BP/BP_FoodOrder.tableNumber` (`self.tableNumber`) _returnvalue)
  (set `/Game/VR_DinnerDash_Assets/BP/BP_FoodOrder.customerWhoOrdered` (`self.customerInTable`) _returnvalue)
  (set `self.foodOrder` _returnvalue))

(fn `UserConstructionScript`)