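; Food station actor for a VR dinner game that turns delivered order actors into table-numbered food items.
; Orders overlapping the receiver collider add their table number to a set-based queue and are destroyed.
; Tick starts one order at a time on a spawn timer, shortened by time accumulated while queued orders waited.
; Spawned food attaches in a spaced row, plays audio, and realigns when an item is removed.
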(event `self.ReceiveTick`
  (params (DeltaSeconds :type "Float (single-precision)"))
  (`self.UpdateOrderQueue` DeltaSeconds))

(event `self.OrderReceiver_Collider.OnComponentBeginOverlap`
  (params (OverlappedComponent :type "PrimitiveComponent Object Reference") (OtherActor :type "Actor Object Reference") (OtherComp :type "PrimitiveComponent Object Reference") (OtherBodyIndex :type Integer) (bFromSweep :type Boolean) (SweepResult :type "HitResult Structure (by ref)"))
  (`self.AddToFoodQueue` OtherActor))

(fn `AddToFoodQueue`
  (params (otherActor :type "Actor Object Reference"))
  (bind _asbp_food_order (cast `/Game/VR_DinnerDash_Assets/BP/BP_FoodOrder` otherActor))
  (`/Engine/EditorBlueprintResources/StandardMacros.IsValid` _asbp_food_order
    (:`Is Valid`
      (`BlueprintSetLibrary.Set_Add` (`self.ordersInQueue`) (`/Game/VR_DinnerDash_Assets/BP/BP_FoodOrder.tableNumber` _asbp_food_order))
      (`self.K2_DestroyActor` otherActor))))

(fn `Remove Food from List`
  (params (FoodItemToRemove :type "/Game/VR_DinnerDash_Assets/BP/BP_FoodItem Object Reference"))
  (`BlueprintSetLibrary.Set_Remove` (`self.listOfFoodItems`) FoodItemToRemove)
  (`self.UpdateLisfOfFood`))

(fn `SpawnFoodItem`
  ;[1 1 1] Spawn Food Item on the station
  (bind _returnvalue (`|SpawnActorFromClass` "/Game/VR_DinnerDash_Assets/BP/BP_FoodItem.BP_FoodItem_C" (`KismetMathLibrary.MakeTransform` (`KismetMathLibrary.MakeVector` (`KismetMathLibrary.Conv_IntToDouble` (+ (`self.foodItemInitialX`) (* (`self.foodItemSpacing`) (`BlueprintSetLibrary.Set_Length` (`self.listOfFoodItems`))))) 0.0 225.0) (struct) (0.5 0.5 0.5)) "Undefined" "OverrideRootScale" null null))
  (`BlueprintSetLibrary.Set_Add` (`self.listOfFoodItems`) _returnvalue)
  (`self.K2_AttachToActor` _returnvalue self "None" "KeepRelative" "KeepRelative" "KeepRelative" true)
  ;;[1 1 1] Set the number in the food item flag to the table number
  (`TextRenderComponent.K2_SetText` (`/Game/VR_DinnerDash_Assets/BP/BP_FoodItem.Table Number` _returnvalue) (`KismetTextLibrary.Conv_IntToText` (`self.currentOrderNumber`)))
  (set `/Game/VR_DinnerDash_Assets/BP/BP_FoodItem.foodStation` self _returnvalue)
  (set `self.OrderInProgress` false)
  (`AudioComponent.Play` (`self.Audio`) 0.0))

(fn `UpdateLisfOfFood`
  ;[1 1 1] Align all food items properly when a food item is grabbed by user
  (bind _result (`BlueprintSetLibrary.Set_ToArray` (`self.listOfFoodItems`)))
  (for (_array_element _array_index) _result
    (`self.K2_SetActorRelativeLocation` _array_element (`KismetMathLibrary.MakeVector` (`KismetMathLibrary.Conv_IntToDouble` (+ (`self.foodItemInitialX`) (* (`self.foodItemSpacing`) _array_index))) 0.0 225.0) false false)))

(fn `UpdateOrderQueue`
  (params (deltaSeconds :type "Float (double-precision)"))
  (bind _foodspawntime (`self.FoodSpawnTime`))
  (bind _ordersinqueue (`self.ordersInQueue`))
  (if (> (`BlueprintSetLibrary.Set_Length` _ordersinqueue) 0)
    (if (not (`self.OrderInProgress`))
      (bind _result (`BlueprintSetLibrary.Set_ToArray` _ordersinqueue))
      (bind _output_get (set `self.currentOrderNumber` (`|GetArrayItem` _result)))
      (`BlueprintSetLibrary.Set_Remove` (`self.ordersInQueue`) _output_get)
      (`KismetSystemLibrary.K2_SetTimer` null "SpawnFoodItem" (`KismetMathLibrary.FClamp` (- _foodspawntime (`self.timePassed`)) 0.0 _foodspawntime))
      (set `self.OrderInProgress` true)
      (set `self.timePassed` 0.0)
      (else
        (set `self.timePassed` (+ deltaSeconds (`self.timePassed`)))))
    (else
      (set `self.timePassed` 0.0))))

(fn `UserConstructionScript`)