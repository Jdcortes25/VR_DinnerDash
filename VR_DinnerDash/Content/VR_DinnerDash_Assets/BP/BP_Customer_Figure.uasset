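; BP_Customer_Figure is a customer figure for the VR Dinner Dash game, built from separate head, body, arm and leg components.
; On BeginPlay it stores the root component's relative transform as InitialTransform.
; HighlightCustomer switches Render Custom Depth on or off for all six body parts to highlight the whole figure.
; The Destroy function is an empty stub, and Tick and overlap events are unused.
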(event `self.ReceiveBeginPlay`
  (set `self.initialTransform` (`SceneComponent.GetRelativeTransform` (`self.RootComponent`))))

(fn `Destroy`)

(fn `HighlightCustomer`
  (params (enableHighlight :type Boolean))
  ;[1 1 1] Highlight all parts of the customer figure
  (`|ExecutionSequence`
    (:`then_0`
      (`PrimitiveComponent.SetRenderCustomDepth` (`self.Head`) enableHighlight))
    (:`then_1`
      (`PrimitiveComponent.SetRenderCustomDepth` (`self.Body`) enableHighlight))
    (:`then_2`
      (`PrimitiveComponent.SetRenderCustomDepth` (`self.Right_Arm`) enableHighlight))
    (:`then_3`
      (`PrimitiveComponent.SetRenderCustomDepth` (`self.Left_Arm`) enableHighlight))
    (:`then_4`
      (`PrimitiveComponent.SetRenderCustomDepth` (`self.Left_Leg`) enableHighlight))
    (:`then_5`
      (`PrimitiveComponent.SetRenderCustomDepth` (`self.Right_Leg`) enableHighlight))))

(fn `UserConstructionScript`)